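; Prototype level tile Blueprint for a runner game that reacts to the PlayerRunner crossing its end plane or hitting its geometry.
; The construction script passes the AttachPoint world transform to SetNextTileTransform, marking where the following tile goes.
; Player overlap with EndPlane calls HandleEndCrossed, while hits on floor, walls or sphere route through HandleCollision to the player's PlaneCollisionComponent as destruction collisions.
; Non-player contacts only print debug strings.
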(event OnComponentBeginOverlap(EndPlane)
  (params (OverlappedComponent :type Primitive%20Component%20Object%20Reference) (OtherActor :type Actor%20Object%20Reference) (OtherComp :type Primitive%20Component%20Object%20Reference) (OtherBodyIndex :type Integer) (bFromSweep :type Boolean) (SweepResult :type Hit%20Result%20Structure%20%28by%20ref%29))
  ;[1 1 1] Endplane Overlap
  (Utilities|Casting|CastToPlayerRunner OtherActor
    (:then
      (Class|TileBase|HandleEndCrossed))
    (:CastFailed
      (Development|PrintString "Something crossed the end plane that isn't the player."))))

(event OnComponentHit(Floor)
  (params (HitComponent :type Primitive%20Component%20Object%20Reference) (OtherActor :type Actor%20Object%20Reference) (OtherComp :type Primitive%20Component%20Object%20Reference) (NormalImpulse :type Vector :default "0, 0, 0") (Hit :type Hit%20Result%20Structure%20%28by%20ref%29))
  ;[1 1 1] Collision
  (CallFunction|HandleCollision HitComponent OtherActor))

(event OnComponentHit(WallR)
  (params (HitComponent :type Primitive%20Component%20Object%20Reference) (OtherActor :type Actor%20Object%20Reference) (OtherComp :type Primitive%20Component%20Object%20Reference) (NormalImpulse :type Vector :default "0, 0, 0") (Hit :type Hit%20Result%20Structure%20%28by%20ref%29))
  ;[1 1 1] Collision
  (CallFunction|HandleCollision HitComponent OtherActor))

(event OnComponentHit(WallL)
  (params (HitComponent :type Primitive%20Component%20Object%20Reference) (OtherActor :type Actor%20Object%20Reference) (OtherComp :type Primitive%20Component%20Object%20Reference) (NormalImpulse :type Vector :default "0, 0, 0") (Hit :type Hit%20Result%20Structure%20%28by%20ref%29))
  ;[1 1 1] Collision
  (CallFunction|HandleCollision HitComponent OtherActor))

(event OnComponentHit(Sphere)
  (params (HitComponent :type Primitive%20Component%20Object%20Reference) (OtherActor :type Actor%20Object%20Reference) (OtherComp :type Primitive%20Component%20Object%20Reference) (NormalImpulse :type Vector :default "0, 0, 0") (Hit :type Hit%20Result%20Structure%20%28by%20ref%29))
  ;[1 1 1] Collision
  (CallFunction|HandleCollision HitComponent OtherActor))

(fn ConstructionScript
  (Class|TileBase|SetNextTileTransform (Transformation|GetWorldTransform (Variables|Default|GetAttachPoint))))

(fn HandleCollision
  (params (Collidee :type Object%20Object%20Reference) (Collider :type Object%20Object%20Reference))
  (bind _asplayer_runner (Utilities|Casting|CastToPlayerRunner Collider)
    (:then
      (Class|PlaneCollisionComponent|OnDestructionCollision (Actor|GetComponentbyClass _asplayer_runner "/Script/ShapeRunner.PlaneCollisionComponent")))
    (:CastFailed
      (Development|PrintString (Utilities|String|ToString(Text) (Utilities|Text|FormatText "{Comp1} Collided with {Comp2}" Collidee Collider))))))
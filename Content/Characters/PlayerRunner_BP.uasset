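; PlayerRunner_BP is the player pawn for a runner game with plane-style flight, possessed by the first player controller on BeginPlay.
; Left and right up/down input actions forward press and release states to PlaneFlightMovement, which handles the flight.
; The construction script sets the initial speed, aligns the camera to the RunnerGameState forward with absolute rotation, then hands it to CameraMovement.
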(event EventBeginPlay
  (Pawn|Possess (Game|GetPlayerController 0) self))

(event Input|ActionEvents|InputActionLeftUpToggle
  (params (Key :type Key%20Structure :default "None"))
  (bind _planeflightmovement (Variables|Default|GetPlaneFlightMovement))
  ;[1 1 1] Keybinding mappings
  (:Pressed
    (Class|PlaneFlightMovementComponent|IntendToggleLeftUpInput _planeflightmovement true))
  (:Released
    (Class|PlaneFlightMovementComponent|IntendToggleLeftUpInput _planeflightmovement false)))

(event Input|ActionEvents|InputActionRightUpToggle
  (params (Key :type Key%20Structure :default "None"))
  (bind _planeflightmovement (Variables|Default|GetPlaneFlightMovement))
  ;[1 1 1] Keybinding mappings
  (:Pressed
    (Class|PlaneFlightMovementComponent|IntendToggleRightUpInput _planeflightmovement true))
  (:Released
    (Class|PlaneFlightMovementComponent|IntendToggleRightUpInput _planeflightmovement false)))

(event Input|ActionEvents|InputActionLeftDownToggle
  (params (Key :type Key%20Structure :default "None"))
  (bind _planeflightmovement (Variables|Default|GetPlaneFlightMovement))
  ;[1 1 1] Keybinding mappings
  (:Pressed
    (Class|PlaneFlightMovementComponent|IntendToggleLeftDownInput _planeflightmovement true))
  (:Released
    (Class|PlaneFlightMovementComponent|IntendToggleLeftDownInput _planeflightmovement false)))

(event Input|ActionEvents|InputActionRightDownToggle
  (params (Key :type Key%20Structure :default "None"))
  (bind _planeflightmovement (Variables|Default|GetPlaneFlightMovement))
  ;[1 1 1] Keybinding mappings
  (:Pressed
    (Class|PlaneFlightMovementComponent|IntendToggleRightDownInput _planeflightmovement true))
  (:Released
    (Class|PlaneFlightMovementComponent|IntendToggleRightDownInput _planeflightmovement false)))

(fn ConstructionScript
  (Variables|/Script/Engine.ProjectileMovementComponent|SetInitialSpeed (Variables|Default|GetPlaneFlightMovement) 1e+03)
  (bind _asrunner_game_state (Utilities|Casting|CastToRunnerGameState (Game|GetGameState)))
  (Transformation|SetWorldRotation (Variables|Default|GetCamera) (Class|RunnerGameState|GetAbsoluteForward _asrunner_game_state) false false)
  (Variables|/Script/Engine.SceneComponent|SetbAbsoluteRotation (Variables|Default|GetCamera) true)
  (Class|CameraMovementComponent|Initialize (Variables|Default|GetCameraMovement) (Variables|Default|GetCamera)))